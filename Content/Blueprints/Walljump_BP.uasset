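; Walljump pad actor that lets the first-person player walljump while overlapping its trigger, provided the pad is not locked.
; On begin overlap it sets the player's CanWalljump state and passes in its per-instance X/Y jump values; end overlap resets the state.
; Tick reapplies a pulsing hex material to the launchpad mesh whenever it is unlocked, showing that the pad is active.
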(event OnComponentBeginOverlap(WalljumpTrigger)
  (params (OverlappedComponent :type Primitive%20Component%20Object%20Reference) (OtherActor :type Actor%20Object%20Reference) (OtherComp :type Primitive%20Component%20Object%20Reference) (OtherBodyIndex :type Integer) (bFromSweep :type Boolean) (SweepResult :type Hit%20Result%20Structure%20%28by%20ref%29))
  (bind _playercharacter (Variables|Default|GetPlayerCharacter))
  ;[1 1 1] Can walljump if adjacent to walljump pad (if active)
  (if (not (Variables|Default|GetIsLocked))
    (Variables|/Game/FirstPersonBP/Blueprints/FirstPersonCharacter.FirstPersonCharacter_C|SetCanWalljump (Variables|Default|GetPlayerCharacter) 2)
    ;;[1 1 1] Each instance has its own WJx/y values
    (Variables|/Game/FirstPersonBP/Blueprints/FirstPersonCharacter.FirstPersonCharacter_C|SetWalljumpX _playercharacter (Variables|Default|GetWalljumpX))
    (Variables|/Game/FirstPersonBP/Blueprints/FirstPersonCharacter.FirstPersonCharacter_C|SetWalljumpY _playercharacter (Variables|Default|GetWalljumpY))))

(event OnComponentEndOverlap(WalljumpTrigger)
  (params (OverlappedComponent :type Primitive%20Component%20Object%20Reference) (OtherActor :type Actor%20Object%20Reference) (OtherComp :type Primitive%20Component%20Object%20Reference) (OtherBodyIndex :type Integer))
  ;[1 1 1] Can walljump if adjacent to walljump pad (if active)
  (Variables|/Game/FirstPersonBP/Blueprints/FirstPersonCharacter.FirstPersonCharacter_C|SetCanWalljump (Variables|Default|GetPlayerCharacter) 1))

(event EventBeginPlay
  (bind _asfirst_person_character (Utilities|Casting|CastToFirstPersonCharacter (Game|GetPlayerCharacter 0)))
  (Variables|Default|SetPlayerCharacter _asfirst_person_character))

(event EventTick
  (params (DeltaSeconds :type Float%20%28single-precision%29))
  ;[1 1 1] If IsLocked is changed to False, material changes to visualize this
  (if (not (Variables|Default|GetIsLocked))
    (Rendering|Material|SetMaterial (Variables|Default|GetLaunchpad) 0 "/Game/StarterContent/Materials/M_Tech_Hex_Tile_Pulse.M_Tech_Hex_Tile_Pulse")))

(fn ConstructionScript)