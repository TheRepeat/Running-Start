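; GunButton_BP is an interactable button that gives the first-person character a gun by setting its HasGun flag.
; BeginPlay caches the player character, and pressing E turns the button light green and sets the flag.
; Entering or leaving the trigger volume enables or disables input on the button and toggles the E prompt text, so the key only works in range.
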(event OnComponentBeginOverlap(InRange_Trigger)
  (params (OverlappedComponent :type Primitive%20Component%20Object%20Reference) (OtherActor :type Actor%20Object%20Reference) (OtherComp :type Primitive%20Component%20Object%20Reference) (OtherBodyIndex :type Integer) (bFromSweep :type Boolean) (SweepResult :type Hit%20Result%20Structure%20%28by%20ref%29))
  ;[1 1 1] Hover text/enable input when in range of button
  (Input|EnableInput (Game|GetPlayerController 0))
  (Rendering|ToggleVisibility (Variables|Default|GetEPromptText) false))

(event OnComponentEndOverlap(InRange_Trigger)
  (params (OverlappedComponent :type Primitive%20Component%20Object%20Reference) (OtherActor :type Actor%20Object%20Reference) (OtherComp :type Primitive%20Component%20Object%20Reference) (OtherBodyIndex :type Integer))
  ;[1 1 1] Hover text/enable input when in range of button
  (Input|DisableInput (Game|GetPlayerController 0))
  (Rendering|ToggleVisibility (Variables|Default|GetEPromptText) false))

(event EventBeginPlay
  (bind _asfirst_person_character (Utilities|Casting|CastToFirstPersonCharacter (Game|GetPlayerCharacter 0)))
  (Variables|Default|SetPlayerCharacter _asfirst_person_character))

(event Input|KeyboardEvents|E
  (params (Key :type Key%20Structure))
  ;[1 1 1] Pressing the button turns on launch pads
  (:Pressed
    (Rendering|Components|Light|SetLightColor (Variables|Default|GetButtonLight) "(R=0.000000,G=1.000000,B=0.000000,A=1.000000)" true)
    (Variables|/Game/FirstPersonBP/Blueprints/FirstPersonCharacter.FirstPersonCharacter_C|SetHasGun (Variables|Default|GetPlayerCharacter) true)))

(fn ConstructionScript)